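; Animatronic enemy that creeps along patrol points toward two doors and triggers a jumpscare game over.
; A looping timer rolls against SpawningValor to teleport it to the next PatrolPath point unless it is scared.
; At the path's end it moves to DoorTarget actors, then either bangs on a closed door or plays the screamer video followed by the GameOver widget.
; ScareAway returns it to the first point and briefly blocks advancing.
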(event `self.ReceiveBeginPlay`
  (`self.SetActorScale3D` (0.15 0.15 0.15))
  (`KismetSystemLibrary.K2_SetTimer` null "MoveToNextSpot" 5.0 true))

(event `play video`
  (bind _returnvalue (`GameplayStatics.GetPlayerController` 0))
  (bind _mediaplayer (`self.Mediaplayer`))
  (set `PlayerController.bShowMouseCursor` false _returnvalue)
  (bind _returnvalue_2 (`|CreateWidget` "/Game/movies/screamer.screamer_C" _returnvalue))
  (`UserWidget.AddToViewport` _returnvalue_2 0)
  (`MediaPlayer.OpenSource` _mediaplayer "/Game/movies/ScreamerSource.ScreamerSource")
  (`MediaPlayer.Play` _mediaplayer)
  (`KismetSystemLibrary.Delay` 2.0)
  (`Widget.RemoveFromParent` _returnvalue_2)
  (set `PlayerController.bShowMouseCursor` true _returnvalue)
  (bind _returnvalue_3 (`|CreateWidget` "/Game/UI/GameOver.GameOver_C" _returnvalue))
  (`UserWidget.AddToViewport` _returnvalue_3 0))

(event `ScareAway`
  (bind (_returnvalue_location _returnvalue_rotation) (`KismetMathLibrary.BreakTransform` (`self.GetTransform` (`|GetArrayItem` (`self.PatrolPath`)))))
  (bind (_returnvalue_location_2 _returnvalue_rotation_2) (`KismetMathLibrary.BreakTransform` (`self.GetTransform` (`|GetArrayItem` (`self.PatrolPath`)))))
  (if (`self.BangingIsPlaying`)
    (`AudioComponent.FadeOut` (`self.doorBangingSound`) 0.5 0.0 "Linear")
    (set `self.IsScared?` true)
    (`self.K2_SetActorTransform` (`KismetMathLibrary.MakeTransform` _returnvalue_location _returnvalue_rotation (0.15 0.15 0.15)))
    (`KismetSystemLibrary.Delay` 5.0)
    (set `self.IsScared?` false)
    (else
      (set `self.IsScared?` true)
      (`self.K2_SetActorTransform` (`KismetMathLibrary.MakeTransform` _returnvalue_location_2 _returnvalue_rotation_2 (0.15 0.15 0.15)))
      (`KismetSystemLibrary.Delay` 5.0)
      (set `self.IsScared?` false))))

(fn `MoveToNextSpot`
  (bind _patrolpath (`self.PatrolPath`))
  (bind _currentindex (`self.CurrentIndex`))
  (bind (_returnvalue_location _returnvalue_rotation) (`KismetMathLibrary.BreakTransform` (`self.GetTransform` (`|GetArrayItem` _patrolpath _currentindex))))
  (`self.SetActorScale3D` (0.15 0.15 0.15))
  (if (< _currentindex (`KismetArrayLibrary.Array_Length` _patrolpath))
    (if (`self.IntheHallway`)
      ; deplacer à la porte la plus proche
      (`self.SetActorScale3D` (0.15 0.15 0.15) :!label _label)
      (for _array_element (`self.DoorTarget`)
        (bind _returnvalue (`KismetMathLibrary.Vector_Distance` (`self.K2_GetActorLocation` _array_element) (`self.K2_GetActorLocation`)))
        (if (< _returnvalue (`self.minDistance`))
          (set `self.minDistance` _returnvalue)
          (bind _output_get (set `self.closestNodes` _array_element))
          (`self.K2_SetActorLocation` (`self.K2_GetActorLocation` _output_get) true)
          (`self.K2_SetActorRotation` (`KismetMathLibrary.FindLookAtRotation` (`self.K2_GetActorLocation`) (`self.K2_GetActorLocation` (`self.closestNodes`))))
          (if (> (`KismetMathLibrary.Vector_Distance` (`self.K2_GetActorLocation` (`self.doorA`)) (`self.K2_GetActorLocation`)) (`KismetMathLibrary.Vector_Distance` (`self.K2_GetActorLocation` (`self.doorB`)) (`self.K2_GetActorLocation`)))
            (set `self.closestNodes` (`self.doorA`))
            (if (`/Game/Blueprints/BP_SecurityDoor.isClosedA` (`self.BP_Door`))
              (if (not (`self.BangingIsPlaying`)) :!label _label_2
                (bind _returnvalue_2 (`GameplayStatics.SpawnSoundAttached` "/Game/sounds/doorBanging.doorBanging" (`self.RootComponent`) "None" (0.0 0.0 0.0) (struct) "KeepRelativeOffset" false 1.0 1.0 0.0 null null false))
                (set `self.doorBangingSound` _returnvalue_2)
                (set `self.BangingIsPlaying` true))
              (else
                (if (`self.BangingIsPlaying`) :!label _label_3
                  (if (not (`self.dead`))
                    (`AudioComponent.FadeOut` (`self.doorBangingSound`) 0.5 0.0 "Linear")
                    (`self.play video`)
                    (set `self.dead` true))
                  (elif (not (`self.dead`))
                    (`self.play video`)
                    (set `self.dead` true)))))
            (else
              (set `self.closestNodes` (`self.doorB`))
              (if (`/Game/Blueprints/BP_SecurityDoor.isClosedB` (`self.BP_Door`))
                (goto _label_2)
                (else
                  (goto _label_3)))))))
      (else
        (if (`self.WasRecentlyRendered` 0.1)
          _
          (else
            _))
        ; level difficulty
        (bind _output_get_2 (set `self.RandomRoll` (`KismetMathLibrary.RandomIntegerInRange` 0 20)))
        (if (< _output_get_2 (`self.spawningValor`))
          (if (not (`self.IsScared?`))
            (`self.K2_SetActorTransform` (`KismetMathLibrary.MakeTransform` _returnvalue_location _returnvalue_rotation (`self.GetActorScale3D`)))
            (`/Engine/EditorBlueprintResources/StandardMacros.IncrementInt` _currentindex
              (:`  `
                (set `self.IntheHallway` (== (`KismetArrayLibrary.Array_Length` (`self.PatrolPath`)) (`self.CurrentIndex`)))
                (if (== (`self.IntheHallway`) true)
                  (goto _label))))))))
    (else
      (set `self.CurrentIndex` 0))))

(fn `UserConstructionScript`)