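; Security door station in a Five Nights at Freddy's-style game, with two clickable doors and two lights for fending off animatronics.
; Button boxes flip-flop each door between timeline-lerped positions and record its closed state.
; Light buttons toggle spotlights, report their state to BP_PlayerController and update power usage.
; Two collision boxes store overlapping animatronics in one shared, never-cleared reference, which either light scares away when switched on.
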(event `self.Box1.OnClicked`
  (params (TouchedComponent :type "PrimitiveComponent Object Reference") (ButtonPressed :type "Key Structure"))
  ; Door
  (`/Engine/EditorBlueprintResources/StandardMacros.FlipFlop`
    (:`A`
      (set `self.isClosedA` true)
      (bind (_direction _alpha) (`Timeline|DoorAnim` :!label _label)
        (:`Update`
          (`SceneComponent.K2_SetRelativeLocation` (`self.DoorPanel`) (`KismetMathLibrary.VLerp` (-384.572338 -5.219908 215.125) (-384.572338 -5.219908 -14.875) _alpha) false false))))
    (:`B`
      (set `self.isClosedA` false)
      (goto _label :!via `Reverse`))))

(event `self.Box.OnClicked`
  (params (TouchedComponent :type "PrimitiveComponent Object Reference") (ButtonPressed :type "Key Structure"))
  ; Door
  (`/Engine/EditorBlueprintResources/StandardMacros.FlipFlop`
    (:`A`
      (set `self.isClosedB` true)
      (bind (_direction _alpha) (`Timeline|Timeline` :!label _label_2)
        (:`Update`
          (`SceneComponent.K2_SetRelativeLocation` (`self.DoorPanel2`) (`KismetMathLibrary.VLerp` (35.427662 -8.219908 215.125) (35.427662 -8.219908 -14.875) _alpha) false false))))
    (:`B`
      (set `self.isClosedB` false)
      (goto _label_2 :!via `Reverse`))))

(event `self.Box2.OnClicked`
  (params (TouchedComponent :type "PrimitiveComponent Object Reference") (ButtonPressed :type "Key Structure"))
  (bind _refenemy_ (`self.RefEnemy `))
  (bind _returnvalue (`SceneComponent.IsVisible` (`self.SpotLight2`)))
  ; Light
  (`SceneComponent.ToggleVisibility` (`self.SpotLight2`) false)
  (bind _asbp_player_controller (cast `/Game/Blueprints/BP_PlayerController` (`GameplayStatics.GetPlayerController` 0)))
  (set `/Game/Blueprints/BP_PlayerController.Light-Box2-On` _returnvalue _asbp_player_controller)
  (`/Game/Blueprints/BP_PlayerController.UpdatePowerUsage` _asbp_player_controller)
  (if _returnvalue
    (`/Engine/EditorBlueprintResources/StandardMacros.IsValid` _refenemy_
      (:`Is Valid`
        (`/Game/Blueprints/BP_Animatronics.ScareAway` _refenemy_)))))

(event `self.Box3.OnClicked`
  (params (TouchedComponent :type "PrimitiveComponent Object Reference") (ButtonPressed :type "Key Structure"))
  (bind _refenemy_ (`self.RefEnemy `))
  (bind _returnvalue (`SceneComponent.IsVisible` (`self.SpotLight1`)))
  ; Light
  (`SceneComponent.ToggleVisibility` (`self.SpotLight1`) false)
  (bind _asbp_player_controller (cast `/Game/Blueprints/BP_PlayerController` (`GameplayStatics.GetPlayerController` 0)))
  (set `/Game/Blueprints/BP_PlayerController.Light-Box3-On` _returnvalue _asbp_player_controller)
  (`/Game/Blueprints/BP_PlayerController.UpdatePowerUsage` _asbp_player_controller)
  (if _returnvalue
    (`/Engine/EditorBlueprintResources/StandardMacros.IsValid` _refenemy_
      (:`Is Valid`
        (`/Game/Blueprints/BP_Animatronics.ScareAway` _refenemy_)))))

(event `self.BoxCollisionB.OnComponentBeginOverlap`
  (params (OverlappedComponent :type "PrimitiveComponent Object Reference") (OtherActor :type "Actor Object Reference") (OtherComp :type "PrimitiveComponent Object Reference") (OtherBodyIndex :type Integer) (bFromSweep :type Boolean) (SweepResult :type "HitResult Structure (by ref)"))
  (bind _asbp_animatronics (cast `/Game/Blueprints/BP_Animatronics` OtherActor))
  (set `self.RefEnemy ` _asbp_animatronics))

(event `self.BoxCollisionA.OnComponentBeginOverlap`
  (params (OverlappedComponent :type "PrimitiveComponent Object Reference") (OtherActor :type "Actor Object Reference") (OtherComp :type "PrimitiveComponent Object Reference") (OtherBodyIndex :type Integer) (bFromSweep :type Boolean) (SweepResult :type "HitResult Structure (by ref)"))
  (bind _asbp_animatronics (cast `/Game/Blueprints/BP_Animatronics` OtherActor))
  (set `self.RefEnemy ` _asbp_animatronics))

(fn `UserConstructionScript`)