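; Player controller for a fixed-position surveillance game with security cameras, doors, lights and a draining battery.
; Creates camera and energy/time widgets, and pans clamped view yaw when the mouse nears screen edges.
; SwitchCamera blends to a chosen feed and sets its post-process weight; Left Shift restores the main view.
; UpdatePowerUsage counts active devices to set a looping timer that drains battery faster for one to three devices.
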(event `self.ReceiveBeginPlay`
  (bind _asbp_character (cast `/Game/Blueprints/BP_Character` (`GameplayStatics.GetPlayerCharacter` 0)))
  (set `self.As BP Character` _asbp_character)
  (set `self.BatteryPercent` 100)
  (set `self.Battery` 100.0)
  (`EnhancedInputSubsystemInterface.AddMappingContext` (subsystem `EnhancedInputLocalPlayerSubsystem`) "/Game/inputs/InputsMappingContext.InputsMappingContext" 1 (struct))
  (set `self.MainCam` (`self.GetViewTarget`))
  ; array Construct for verification
  (`KismetArrayLibrary.Array_Append` (`self.CameraList`) (`|MakeArray` (`self.CamB`) (`self.CamA`) (`self.Cam8`) (`self.Cam7`) (`self.Cam6`) (`self.Cam5`) (`self.Cam4`) (`self.Cam3`) (`self.Cam2`) (`self.Cam1`)))
  ; init UI Camera
  (bind _returnvalue (`|CreateWidget` "/Game/UI/camera/cameraUI.cameraUI_C" null (`self.Cam1`) (`self.Cam2`) (`self.Cam3`) (`self.Cam4`) (`self.Cam5`) (`self.Cam6`) (`self.Cam7`) (`self.Cam8`) (`self.CamA`) (`self.CamB`)))
  (set `self.CameraUI` _returnvalue)
  (`UserWidget.AddToViewport` _returnvalue 0)
  (set `self.bShowMouseCursor` true)
  (`WidgetBlueprintLibrary.SetInputMode_GameAndUIEx` (`GameplayStatics.GetPlayerController` 0) _returnvalue "DoNotLock" false)
  (bind _returnvalue_2 (`|CreateWidget` "/Game/UI/energyandtime/BP_energyAndTime.BP_energyAndTime_C"))
  (bind _output_get (set `self.Horloge` _returnvalue_2))
  (`UserWidget.AddToViewport` _output_get 0))

(event `self.ReceiveTick`
  (params (DeltaSeconds :type "Float (single-precision)"))
  (bind _returnvalue_x (`KismetMathLibrary.BreakVector2D` (`WidgetLayoutLibrary.GetViewportSize`)))
  (bind (_returnvalue_roll _returnvalue_pitch _returnvalue_yaw) (`KismetMathLibrary.BreakRotator` (`self.GetControlRotation`)))
  (bind _returnvalue (/ (`self.GetMousePosition`) _returnvalue_x))
  ; Camera
  (if (< _returnvalue 0.1)
    (`self.SetControlRotation` (`KismetMathLibrary.MakeRotator` _returnvalue_roll _returnvalue_pitch (`KismetMathLibrary.FClamp` (- _returnvalue_yaw 1.0) -150.0 -30.0)))
    (elif (> _returnvalue 0.9)
      (`self.SetControlRotation` (`KismetMathLibrary.MakeRotator` _returnvalue_roll _returnvalue_pitch (`KismetMathLibrary.FClamp` (+ _returnvalue_yaw 1.0) -150.0 -30.0))))))

(event `Key|LeftShift`
  (params (Key :type "Key Structure"))
  (:`Pressed`
    (`self.SetViewTargetWithBlend` (`self.MainCam`))
    (set `self.IsCameraOpen?` false)
    (for _array_element (`self.CameraList`)
      (`CameraComponent.SetPostProcessBlendWeight` (`CameraActor.CameraComponent` _array_element) 0.0))
    (`Widget.SetVisibility` (`/Game/UI/camera/cameraUI.Second-UI` (`self.CameraUI`)) "Collapsed")))

(event `UpdatePowerUsage`
  ; Battery
  (`KismetSystemLibrary.K2_ClearAndInvalidateTimerHandle` (`self.BatteryTimerHandle`))
  (switch `int` (+ (`KismetMathLibrary.SelectInt` 1 0 (`self.IsCameraOpen?`)) (`KismetMathLibrary.SelectInt` 1 0 (`self.DoorA-On`)) (`KismetMathLibrary.SelectInt` 1 0 (`self.DoorB-On`)) (`KismetMathLibrary.SelectInt` 1 0 (`self.Light-Box2-On`)) (`KismetMathLibrary.SelectInt` 1 0 (`self.Light-Box3-On`)))
    (:`1`
      (bind _returnvalue (`KismetSystemLibrary.K2_SetTimerDelegate` (delegate `LowBattery`) 6.0 true))
      (set `self.BatteryTimerHandle` _returnvalue))
    (:`2`
      (bind _returnvalue_2 (`KismetSystemLibrary.K2_SetTimerDelegate` (delegate `LowBattery`) 3.0 true))
      (set `self.BatteryTimerHandle` _returnvalue_2))
    (:`3`
      (bind _returnvalue_3 (`KismetSystemLibrary.K2_SetTimerDelegate` (delegate `LowBattery`) 1.0 true))
      (set `self.BatteryTimerHandle` _returnvalue_3))))

(event `LowBattery`
  ; Battery
  (bind _output_get (set `self.BatteryPercent` (`KismetMathLibrary.Clamp` (- (`self.BatteryPercent`) 1) 0 100)))
  (bind _output_get_2 (set `self.Battery` (`KismetMathLibrary.Conv_IntToDouble` _output_get)))
  (`self.UpdateBatteryUI` (`KismetMathLibrary.FTrunc` _output_get_2)))

(fn `SwitchCamera`
  (params (TargetCamera :type "CameraActor Object Reference"))
  ; verification active camera
  (bind _output_get (set `self.activeCam` TargetCamera))
  (for _array_element (`self.CameraList`)
    (if (== (`self.activeCam`) _array_element)
      (`ActorComponent.Activate` (`Actor.RootComponent` _array_element) false :!label _label)
      (for _array_element_2 (`self.CameraList`)
        (`CameraComponent.SetPostProcessBlendWeight` (`CameraActor.CameraComponent` _array_element_2) 0.0))
      (`self.SetViewTargetWithBlend` TargetCamera)
      (set `self.IsCameraOpen?` true)
      (bind _cameracomponent (`CameraActor.CameraComponent` _output_get))
      (if (!= _cameracomponent (`/Game/Blueprints/BP_Character.Camera` (`self.As BP Character`)))
        (`CameraComponent.SetPostProcessBlendWeight` _cameracomponent 1.0)
        (else
          (`CameraComponent.SetPostProcessBlendWeight` _cameracomponent 0.0)))
      (else
        (`ActorComponent.Deactivate` (`Actor.RootComponent` _array_element)))))
  (goto _label))

(fn `UserConstructionScript`)